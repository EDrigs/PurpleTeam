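; Red ability ammo pickup that tops up the first-person character's Malware or Ransomware ammo when the player overlaps its capsule.
; A random pick chooses which ammo to add, falling back to the other type if that one is maxed.
; Unless both are full, it plays a sound, then hides and disables collision.
; Ending the overlap starts a fixed delay that restores visibility and collision, acting as a respawn.
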(event OnComponentBeginOverlap(Capsule)
  (params (OverlappedComponent :type Primitive%20Component%20Object%20Reference) (OtherActor :type Actor%20Object%20Reference) (OtherComp :type Primitive%20Component%20Object%20Reference) (OtherBodyIndex :type Integer) (bFromSweep :type Boolean) (SweepResult :type Hit%20Result%20Structure%20%28by%20ref%29))
  ;[1 1 1] Item Pickup: Increments counter on Character BP, if counter below threshold continue, hides item, turns off collision
  (bind _asbp_first_person_character (Utilities|Casting|CastToBP_FirstPersonCharacter OtherActor))
  (Variables|Default|SetisRedAmmoMaxed false)
  (switch int (Math|Random|RandomIntegerinRange 0 1)
    (:0
      (CallFunction|SetMalwareAmmo _asbp_first_person_character))
    (:1
      (CallFunction|SetRansomwareAmmo _asbp_first_person_character)))
  (if (not (Variables|Default|GetisRedAmmoMaxed))
    (Audio|PlaySound2D "/Engine/VREditor/Sounds/UI/Camera_Shutter.Camera_Shutter" 1.0 1.0 0.0 0 0)
    (Rendering|SetActorHiddenInGame true)
    (Collision|SetActorEnableCollision false)))

(event OnComponentEndOverlap(Capsule)
  (params (OverlappedComponent :type Primitive%20Component%20Object%20Reference) (OtherActor :type Actor%20Object%20Reference) (OtherComp :type Primitive%20Component%20Object%20Reference) (OtherBodyIndex :type Integer))
  ;[1 1 1] Item Respawn: starts timer, unhides actor, turns on collision
  (Utilities|FlowControl|Delay 3e+01)
  (Rendering|SetActorHiddenInGame false)
  (Collision|SetActorEnableCollision true))

(event EventBeginPlay)

(event Collision|EventActorBeginOverlap
  (params (OtherActor :type Actor%20Object%20Reference)))

(event EventTick
  (params (DeltaSeconds :type Float%20%28single-precision%29)))

(fn ConstructionScript)

(fn SetMalwareAmmo
  (params (Target :type BP%20First%20Person%20Character%20Object%20Reference))
  (if (< (Variables|/Game/FirstPerson/Blueprints/BP_FirstPersonCharacter.BP_FirstPersonCharacter_C|GetmalwareAmmo Target) (Variables|/Game/FirstPerson/Blueprints/BP_FirstPersonCharacter.BP_FirstPersonCharacter_C|GetmalwareMaxAmmo Target))
    (Variables|/Game/FirstPerson/Blueprints/BP_FirstPersonCharacter.BP_FirstPersonCharacter_C|SetmalwareAmmo Target (+ (Variables|/Game/FirstPerson/Blueprints/BP_FirstPersonCharacter.BP_FirstPersonCharacter_C|GetmalwareAmmo Target) 5))
    (Default|PickupRed Target)
    (else
      (CallFunction|SetRansomwareAmmo Target))))

(fn SetRansomwareAmmo
  (params (self2 :type BP%20First%20Person%20Character%20Object%20Reference))
  (if (< (Variables|/Game/FirstPerson/Blueprints/BP_FirstPersonCharacter.BP_FirstPersonCharacter_C|GetransomwareAmmo self2) (Variables|/Game/FirstPerson/Blueprints/BP_FirstPersonCharacter.BP_FirstPersonCharacter_C|GetransomwareMaxAmmo self2))
    (Variables|/Game/FirstPerson/Blueprints/BP_FirstPersonCharacter.BP_FirstPersonCharacter_C|SetransomwareAmmo self2 (+ (Variables|/Game/FirstPerson/Blueprints/BP_FirstPersonCharacter.BP_FirstPersonCharacter_C|GetransomwareAmmo self2) 1))
    (Default|PickupRed self2)
    (elif (< (Variables|/Game/FirstPerson/Blueprints/BP_FirstPersonCharacter.BP_FirstPersonCharacter_C|GetmalwareAmmo self2) (Variables|/Game/FirstPerson/Blueprints/BP_FirstPersonCharacter.BP_FirstPersonCharacter_C|GetmalwareMaxAmmo self2))
      (CallFunction|SetMalwareAmmo self2)
      (else
        (Variables|Default|SetisRedAmmoMaxed true)))))