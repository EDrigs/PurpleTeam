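; BP_AbilityPickup is a respawning pickup that grants the first-person character one ability charge, up to a cap.
; Capsule begin overlap increments the character's NumAbility, plays a sound and explosion effect, then hides the actor and disables its collision.
; Capsule end overlap, unfiltered by actor or pickup success, starts a fixed delay that unhides the actor and restores collision.
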(event OnComponentBeginOverlap(Capsule)
  (params (OverlappedComponent :type Primitive%20Component%20Object%20Reference) (OtherActor :type Actor%20Object%20Reference) (OtherComp :type Primitive%20Component%20Object%20Reference) (OtherBodyIndex :type Integer) (bFromSweep :type Boolean) (SweepResult :type Hit%20Result%20Structure%20%28by%20ref%29))
  ;[1 1 1] Item Pickup: Increments counter on Character BP, if counter below threshold continue, hides item, turns off collision
  (bind _asbp_first_person_character (Utilities|Casting|CastToBP_FirstPersonCharacter OtherActor))
  (if (< (Variables|/Game/FirstPerson/Blueprints/BP_FirstPersonCharacter.BP_FirstPersonCharacter_C|GetnumAbility%20 _asbp_first_person_character) 5)
    (Variables|/Game/FirstPerson/Blueprints/BP_FirstPersonCharacter.BP_FirstPersonCharacter_C|SetnumAbility%20 _asbp_first_person_character (+ (Variables|/Game/FirstPerson/Blueprints/BP_FirstPersonCharacter.BP_FirstPersonCharacter_C|GetnumAbility%20 _asbp_first_person_character) 1))
    (Audio|PlaySound2D "/Engine/VREditor/Sounds/UI/Camera_Shutter.Camera_Shutter" 1.0 1.0 0.0 0 0)
    (Effects|SpawnEmitteratLocation "/Game/StarterContent/Particles/P_Explosion.P_Explosion" (Transformation|GetActorLocation self))
    (Rendering|SetActorHiddenInGame true)
    (Collision|SetActorEnableCollision false)))

(event OnComponentEndOverlap(Capsule)
  (params (OverlappedComponent :type Primitive%20Component%20Object%20Reference) (OtherActor :type Actor%20Object%20Reference) (OtherComp :type Primitive%20Component%20Object%20Reference) (OtherBodyIndex :type Integer))
  ;[1 1 1] Item Respawn: starts timer, unhides actor, turns on collision
  (Utilities|FlowControl|Delay 3e+01)
  (Rendering|SetActorHiddenInGame false)
  (Collision|SetActorEnableCollision true))

(event EventBeginPlay)

(event Collision|EventActorBeginOverlap
  (params (OtherActor :type Actor%20Object%20Reference)))

(event EventTick
  (params (DeltaSeconds :type Float%20%28single-precision%29)))

(fn ConstructionScript)