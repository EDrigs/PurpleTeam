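; Waypoint marker actor that shows a distance readout on its Waypoint widget.
; BeginPlay casts the widget component's widget to Waypoint and caches its DistanceText.
; Every Tick sets that text from CalculateDistanceText, whose nodes turn the actor-to-player-pawn distance into truncated meters with an "m" suffix.
; That calculation appears unconnected to any function output in the graph.
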(event EventBeginPlay
  (bind _aswaypoint (Utilities|Casting|CastToWaypoint (UserInterface|GetWidget (Variables|Default|GetWidget))))
  (Variables|Default|SetDistance%20Text (Variables|/Game/Objectives/Blueprints/Waypoint.Waypoint_C|GetDistanceText _aswaypoint)))

(event EventTick
  (params (DeltaSeconds :type Float%20%28single-precision%29))
  (Rendering|Components|TextRender|SetText (Variables|Default|GetDistance%20Text) (|CalculateDistanceText)))

(fn ConstructionScript)