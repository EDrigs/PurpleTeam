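; AI controller for the Time and Space ability pack that makes AI awareness of the player respect the invisibility ability.
; On BeginPlay it runs AI_Tree and starts a looping one-second timer that polls perception for player 0.
; When the player is among known perceived actors and has an AC_Invisible component, it sets the "CanSeePlayer?" blackboard key to the inverse of IsInvisibleActive.
; Otherwise the key is left unchanged.
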(event EventBeginPlay
  (AI|RunBehaviorTree "/Game/Assets/AbilityPack-TimeAndSpace/Blueprints/AI/AI_Tree.AI_Tree")
  (Utilities|Time|SetTimerbyFunctionName 0 "UpdateTarget" 1.0 true))

(fn ConstructionScript)

(fn UpdateTarget
  (bind _returnvalue (Game|GetPlayerCharacter 0))
  (if (Utilities|Array|ContainsItem (Class|AIPerceptionComponent|GetKnownPerceivedActors (Variables|Default|GetAIPerception)) _returnvalue)
    (bind _asbp_character (Utilities|Casting|CastToBP_Character _returnvalue))
    (Utilities|IsValid (Actor|GetComponentbyClass _asbp_character "/Game/Assets/AbilityPack-TimeAndSpace/Blueprints/Components/AC_Invisible.AC_Invisible_C")
      (:Is%20Valid
        (AI|Components|Blackboard|SetValueasBool (AI|GetBlackboard 0) (Utilities|Name|MakeLiteralName "CanSeePlayer?") (not (Variables|/Game/Assets/AbilityPack-TimeAndSpace/Blueprints/Components/AC_Invisible.AC_Invisible_C|GetIsInvisibleActive? (Actor|GetComponentbyClass _asbp_character "/Game/Assets/AbilityPack-TimeAndSpace/Blueprints/Components/AC_Invisible.AC_Invisible_C"))))))))